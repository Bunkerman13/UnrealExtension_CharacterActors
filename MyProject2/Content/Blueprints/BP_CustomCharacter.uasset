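; BP_CustomCharacter is a character Blueprint that displays its health on a HUD.
; On BeginPlay it creates WBP_HUD, stores the reference and adds it to the viewport.
; BeginPlay and AnyDamage share a validity-checked update that passes current and default health from CustomHealth to the HUD.
; The graph only refreshes the display and does not change health itself.
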(event EventBeginPlay
  (bind _customhealth (Variables|Default|GetCustomHealth))
  (bind _returnvalue (UserInterface|CreateWidget "/Game/Blueprints/Widgets/WBP_HUD.WBP_HUD_C"))
  (bind _output_get (Variables|Default|SetHUDRef _returnvalue))
  (UserInterface|Viewport|AddtoViewport _output_get 0)
  (Utilities|IsValid (Variables|Default|GetHUDRef)
    (:Is%20Valid
      (Default|UpdateHealth (Variables|Default|GetHUDRef) (Variables|/Script/MyProject2.CustomHealthComponent|GetHealth _customhealth) (Variables|/Script/MyProject2.CustomHealthComponent|GetDefaultHealth _customhealth)))))

(event Collision|EventActorBeginOverlap
  (params (OtherActor :type Actor%20Object%20Reference)))

(event EventTick
  (params (DeltaSeconds :type Float%20%28single-precision%29)))

(event Game|Damage|EventAnyDamage
  (params (Damage :type Float%20%28single-precision%29) (DamageType :type Damage%20Type%20Object%20Reference) (InstigatedBy :type Controller%20Object%20Reference) (DamageCauser :type Actor%20Object%20Reference))
  (bind _customhealth (Variables|Default|GetCustomHealth))
  (Utilities|IsValid (Variables|Default|GetHUDRef)
    (:Is%20Valid
      (Default|UpdateHealth (Variables|Default|GetHUDRef) (Variables|/Script/MyProject2.CustomHealthComponent|GetHealth _customhealth) (Variables|/Script/MyProject2.CustomHealthComponent|GetDefaultHealth _customhealth)))))

(fn ConstructionScript)